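; BP_Badguy1 is an enemy AI character that roams randomly, chases pawns it sees and attacks them with a punch montage.
; PawnSensing interrupts roaming with a move toward the seen pawn and a gated punch, then a retriggerable delay restarts roaming.
; AttackPunch overlaps apply damage to BP_ThirdPersonCharacter while Attack is true, though this graph never sets that flag.
; Incoming damage sets Health to Damage minus Health and prints it, with no death handling.
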(event `self.ReceiveBeginPlay`
  (`self.Random Roam`))

(event `Random Roam`
  (`|AIMoveTo` self (`NavigationSystemV1.K2_GetRandomReachablePointInRadius` (`self.K2_GetActorLocation`) 1500.0 null null) null 70.0 true
    (:`OnSuccess`
      (`self.Random Roam`))))

(event `self.PawnSensing.OnSeePawn`
  (params (Pawn :type "Pawn Object Reference"))
  (set `self.Can Attack` true)
  (`|ExecutionSequence`
    (:`then_0`
      (`|AIMoveTo` self (0.0 0.0 0.0) Pawn 70.0 true
        (:`then`
          (if (`self.Can Attack`)
            (`/Engine/EditorBlueprintResources/StandardMacros.DoOnce` false :!label _label
              (:`Completed`
                (set `self.Can Attack` false)
                (bind _returnvalue (`self.PlayAnimMontage` "/Game/Characters/enemyAI/all_anims_for_badguys/badguy1/AttackPunch.AttackPunch"))
                (`KismetSystemLibrary.Delay` _returnvalue)
                (goto _label :!via `Reset`)))))))
    (:`then_1`
      (`KismetSystemLibrary.RetriggerableDelay` 1.0)
      (`self.Random Roam`))))

(event `self.AttackPunch.OnComponentBeginOverlap`
  (params (OverlappedComponent :type "PrimitiveComponent Object Reference") (OtherActor :type "Actor Object Reference") (OtherComp :type "PrimitiveComponent Object Reference") (OtherBodyIndex :type Integer) (bFromSweep :type Boolean) (SweepResult :type "HitResult Structure (by ref)"))
  ; Dmg Dealt
  (bind _asbp_third_person_character (cast `/Game/ThirdPerson/Blueprints/BP_ThirdPersonCharacter` OtherActor)
    (:`then`
      _)
    (:`CastFailed`
      _))
  (if (`self.Attack`)
    (`/Engine/EditorBlueprintResources/StandardMacros.DoOnce` false :!label _label_2
      (:`Completed`
        (bind _returnvalue (`GameplayStatics.ApplyDamage` _asbp_third_person_character 0.15))
        (`KismetSystemLibrary.Delay` _returnvalue)
        (goto _label_2 :!via `Reset`)))))

(event `self.ReceiveAnyDamage`
  (params (Damage :type "Float (single-precision)") (DamageType :type "DamageType Object Reference") (InstigatedBy :type "Controller Object Reference") (DamageCauser :type "Actor Object Reference"))
  ; Dmg Taken
  (bind _output_get (set `self.Health` (- Damage (`self.Health`))))
  (`KismetSystemLibrary.PrintString` (`KismetStringLibrary.Conv_DoubleToString` _output_get)))

(fn `UserConstructionScript`)